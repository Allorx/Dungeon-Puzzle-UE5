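; BPWeapon is a weapon actor that deals damage to Object_A actors it overlaps.
; On overlap it ignores itself, casts the other actor to Object_A and calls its Damage function with the attack damage and damage type.
; The damage origin is the attach parent's location, so the weapon expects to be attached to another actor.
; The returned result only selects a hit or miss debug print.
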(event EventBeginPlay)

(event Collision|EventActorBeginOverlap
  (params (OtherActor :type Actor%20Object%20Reference))
  ;[0 0.547 1] When this overlaps an Object_A damage is dealt to the Object_A
  (if (!= OtherActor self)
    (bind _asobject_a (Utilities|Casting|CastToObject_A OtherActor))
    (bind _returnvalue (Class|ObjectA|Damage _asobject_a (Variables|Default|GetAttackDamage) (Variables|Default|GetDamageType) (Transformation|GetActorLocation (Actor|GetAttachParentActor))))
    (if _returnvalue
      (Development|PrintString "Hit!")
      (else
        (Development|PrintString "Nop")))))

(event EventTick
  (params (DeltaSeconds :type Float%20%28single-precision%29)))

(fn ConstructionScript)