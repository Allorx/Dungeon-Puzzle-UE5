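; Main player Blueprint with a camera, which looks up and caches key level actors at startup.
; On BeginPlay it finds a Cube_A actor as HitActor and a MainChar_Object_A actor as MainCharacter.
; The mouse wheel axis event is empty.
; A disconnected zoom branch would offset the camera along X between zoom limits, with a note that it sometimes leaves those bounds and stops working.
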(event EventBeginPlay
  (bind _returnvalue (Actor|GetActorOfClass "/Script/DungeonGame.Cube_A"))
  (Variables|Default|SethitActor _returnvalue)
  (bind _returnvalue_2 (Actor|GetActorOfClass "/Script/DungeonGame.MainChar_Object_A"))
  (Variables|Default|SetmainCharacter _returnvalue_2))

(event Input|MouseEvents|MouseWheelAxis
  (params (AxisValue :type Float%20%28single-precision%29)))

(fn ConstructionScript)